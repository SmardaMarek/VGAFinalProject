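; BP_NPC is a talkable NPC that shows its dialog lines one at a time.
; Each Talk call advances an index, creates a WB_Dialog widget on first use, sets its text and plays a sound.
; Past the last line, it removes the widget and resets the index so the conversation can start over.
; A separate event destroys the NPC.
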(event Custom|Event%20DeleteNPC
  ;[0.15 0.15 0.15 0.5] Delete
  (Actor|DestroyActor))

(event EventRestartDialog
  ;[0.15 0.15 0.15 0.5] Reset Dialog
  (Widget|RemovefromParent (Variables|Default|GetUI))
  (Variables|Default|SetUI 0)
  (Variables|Default|SetTalkIndex -1))

(event EventTalk
  ;[0.15 0.15 0.15 0.5] Talk
  (Math|Integer|IncrementInt (Variables|Default|GetTalkIndex)
    (:%20%20
      (if (< (Variables|Default|GetTalkIndex) (Utilities|Array|Length (Variables|Default|GetDialog)))
        (Variables|Default|GetUI
          (:then
            _)
          (:else
            (bind _returnvalue (UserInterface|CreateWidget "/Game/NPC/WB_Dialog.WB_Dialog_C" (Game|GetPlayerController 0)))
            (bind _output_get (Variables|Default|SetUI _returnvalue))
            (UserInterface|Viewport|AddtoViewport _output_get 0)))
        (Rendering|Components|TextRender|SetText (Variables|/Game/NPC/WB_Dialog.WB_Dialog_C|GetTalkText (Variables|Default|GetUI)) (Utilities|Text|ToText(String) (Utilities|Array|Get(acopy) (Variables|Default|GetDialog) (Variables|Default|GetTalkIndex))))
        (Audio|PlaySound2D "/Engine/EditorSounds/Notifications/CompileSuccess.CompileSuccess" 1.0 1.0 0.0 0 0)
        (else
          (CallFunction|RestartDialog))))))

(fn ConstructionScript)